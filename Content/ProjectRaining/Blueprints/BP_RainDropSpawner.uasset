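; BP_RainDropSpawner is an actor that turns an impact into a water splash and a scattering of raindrop pickups.
; The first hit on its Plane component passes a DoOnce, which is never reset here, and spawns a vertical splash emitter at the actor's location.
; After a short delay, it spawns a small random number of BP_RainDrop_Pickup actors at random horizontal offsets around that location.
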(event OnComponentHit(Plane)
  (params (HitComponent :type Primitive%20Component%20Object%20Reference) (OtherActor :type Actor%20Object%20Reference) (OtherComp :type Primitive%20Component%20Object%20Reference) (NormalImpulse :type Vector :default "0, 0, 0") (Hit :type Hit%20Result%20Structure%20%28by%20ref%29))
  (bind _plane (Variables|Default|GetPlane))
  (bind _returnvalue (Components|GetOwner _plane))
  (bind _returnvalue_2 (Transformation|GetActorLocation _returnvalue))
  (Utilities|FlowControl|DoOnce false
    (:Completed
      (Effects|SpawnEmitteratLocation "/Game/InfinityBladeEffects/Effects/FX_Ambient/Water/P_Water_Splash_Vertical.P_Water_Splash_Vertical" _returnvalue_2)
      (Utilities|FlowControl|Delay 0.5)
      (bind _output_get (Variables|Default|SetRandomMeshAmount (Math|Random|RandomIntegerinRange 1 7)))
      (for _index (range 0 _output_get)
        (Game|SpawnActorfromClass "/Game/ProjectRaining/Blueprints/BP_RainDrop_Pickup.BP_RainDrop_Pickup_C" (Math|Conversions|ToTransform(Vector) (+ (Math|Vector|MakeVector (Math|Random|RandomFloatinRange -1.5e+02 1.5e+02) (Math|Random|RandomFloatinRange -1.5e+02 1.5e+02) 0.0) _returnvalue_2)) "Undefined" 0 0)))))

(fn ConstructionScript)