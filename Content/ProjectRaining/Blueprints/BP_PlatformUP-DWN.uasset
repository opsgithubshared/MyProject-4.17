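; BP_PlatformUP-DWN is a moving platform that travels between two points when the player triggers it.
; On BeginPlay it caches the Platform and End component world locations as start and end points and sets the timeline play rate from a variable.
; A PlayerCharacter overlapping AreaCollide plays the timeline, which lerps the platform's world location toward the end point without sweeping.
; The graph has no reverse or end-overlap logic.
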(event OnComponentBeginOverlap(AreaCollide)
  (params (OverlappedComponent :type Primitive%20Component%20Object%20Reference) (OtherActor :type Actor%20Object%20Reference) (OtherComp :type Primitive%20Component%20Object%20Reference) (OtherBodyIndex :type Integer) (bFromSweep :type Boolean) (SweepResult :type Hit%20Result%20Structure%20%28by%20ref%29))
  (Utilities|Casting|CastToPlayerCharacter OtherActor)
  (bind _playrate (Timeline|Platform_Mov Play)
    (:Update
      (Transformation|SetWorldLocation (Variables|Default|GetPlatform) (Math|Vector|Lerp(Vector) (Variables|Default|GetStart_Point) (Variables|Default|GetEnd_Point) _playrate) false false))))

(event EventBeginPlay
  (CallFunction|SetLocations))

(fn ConstructionScript)

(fn SetLocations
  (Variables|Default|SetStart_Point (Transformation|GetWorldLocation (Variables|Default|GetPlatform)))
  (Variables|Default|SetEnd_Point (Transformation|GetWorldLocation (Variables|Default|GetEnd)))
  (Components|Timeline|SetPlayRate (Variables|Default|GetPlatform_Mov) (Variables|Default|GetPlayrate)))