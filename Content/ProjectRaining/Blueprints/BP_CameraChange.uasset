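; Trigger actor that switches the player character between its top-down and side-view cameras through two overlap components.
; The top overlap activates TopDownCamera, initializes FadeCameraOccluders between that camera and the character's Scene, and deactivates SideViewCamera.
; The front overlap reverses the cameras and also deactivates Scene.
; A boolean prevents repeat switches; overlaps always target player 0 without checking the overlapping actor.
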(event OnComponentBeginOverlap(cameratop)
  (params (OverlappedComponent :type Primitive%20Component%20Object%20Reference) (OtherActor :type Actor%20Object%20Reference) (OtherComp :type Primitive%20Component%20Object%20Reference) (OtherBodyIndex :type Integer) (bFromSweep :type Boolean) (SweepResult :type Hit%20Result%20Structure%20%28by%20ref%29))
  (if (not (Variables|Default|GetCameraTop))
    (bind _asplayer_character (Utilities|Casting|CastToPlayerCharacter (Game|GetPlayerCharacter 0)))
    (Components|Activation|SetActive (Variables|/Game/ProjectRaining/Characters/PlayerCharacter/PlayerCharacter.PlayerCharacter_C|GetTopDownCamera _asplayer_character) true false)
    (Default|Init (Variables|/Game/ProjectRaining/Characters/PlayerCharacter/PlayerCharacter.PlayerCharacter_C|GetFadeCameraOccluders _asplayer_character) (Variables|/Game/ProjectRaining/Characters/PlayerCharacter/PlayerCharacter.PlayerCharacter_C|GetTopDownCamera _asplayer_character) (Variables|/Game/ProjectRaining/Characters/PlayerCharacter/PlayerCharacter.PlayerCharacter_C|GetScene _asplayer_character))
    (Components|Activation|SetActive (Variables|/Game/ProjectRaining/Characters/PlayerCharacter/PlayerCharacter.PlayerCharacter_C|GetSideViewCamera _asplayer_character) false false)
    (Variables|Default|SetCameraTop true)))

(event OnComponentBeginOverlap(camerafront)
  (params (OverlappedComponent :type Primitive%20Component%20Object%20Reference) (OtherActor :type Actor%20Object%20Reference) (OtherComp :type Primitive%20Component%20Object%20Reference) (OtherBodyIndex :type Integer) (bFromSweep :type Boolean) (SweepResult :type Hit%20Result%20Structure%20%28by%20ref%29))
  (if (Variables|Default|GetCameraTop)
    (bind _asplayer_character (Utilities|Casting|CastToPlayerCharacter (Game|GetPlayerCharacter 0)))
    (Components|Activation|SetActive (Variables|/Game/ProjectRaining/Characters/PlayerCharacter/PlayerCharacter.PlayerCharacter_C|GetTopDownCamera _asplayer_character) false false)
    (Components|Activation|SetActive (Variables|/Game/ProjectRaining/Characters/PlayerCharacter/PlayerCharacter.PlayerCharacter_C|GetSideViewCamera _asplayer_character) true false)
    (Variables|Default|SetCameraTop false)))

(fn ConstructionScript)